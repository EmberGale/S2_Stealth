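; Pin code panel actor for the stealth section that opens the HUD's PIN entry UI while the player character stands inside its sphere trigger and closes it on exit.
; Shortly after BeginPlay it binds to the HUD_Player pin code widget's success event.
; A successful entry sends TriggerMessage to its ActorsToTrigger, leaving the code check itself to the widget.
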(event OnComponentBeginOverlap(Sphere)
  (params (OverlappedComponent :type Primitive%20Component%20Object%20Reference) (OtherActor :type Actor%20Object%20Reference) (OtherComp :type Primitive%20Component%20Object%20Reference) (OtherBodyIndex :type Integer) (bFromSweep :type Boolean) (SweepResult :type Hit%20Result%20Structure%20%28by%20ref%29))
  (if (== OtherActor (Game|GetPlayerCharacter 0))
    (bind _ashud_player (Utilities|Casting|CastToHUD_Player (HUD|GetHUD (Game|GetPlayerController 0))))
    (Default|OpenPIN-codePanel _ashud_player)))

(event OnComponentEndOverlap(Sphere)
  (params (OverlappedComponent :type Primitive%20Component%20Object%20Reference) (OtherActor :type Actor%20Object%20Reference) (OtherComp :type Primitive%20Component%20Object%20Reference) (OtherBodyIndex :type Integer))
  (if (== OtherActor (Game|GetPlayerCharacter 0))
    (bind _ashud_player (Utilities|Casting|CastToHUD_Player (HUD|GetHUD (Game|GetPlayerController 0))))
    (Default|ClosePIN-codePanel _ashud_player)))

(event Custom|OnSuccess_Event
  (Class|BPITrigger|Trigger(Message) (Variables|Default|GetActorsToTrigger)))

(event EventBeginPlay
  (Utilities|FlowControl|Delay 0.2)
  (bind _ashud_player (Utilities|Casting|CastToHUD_Player (HUD|GetHUD (Game|GetPlayerController 0))))
  (EventDispatchers|AssignOnSuccess (Variables|/Game/S2_Stealth/PlayerLogic/HUD_Player.HUD_Player_C|GetWB_UI_PinCode _ashud_player) (delegate Custom|OnSuccess_Event)))

(fn ConstructionScript)