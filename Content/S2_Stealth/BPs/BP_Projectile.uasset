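; BP_Projectile is a configurable projectile actor for the stealth section that damages what it hits.
; The construction script applies the Mesh, location offset and rotation variables to its static mesh.
; A hit on the Sphere component applies Damage to the other actor.
; The DestroyActor node is unconnected, so this graph does not destroy the projectile on impact.
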(event OnComponentHit(Sphere)
  (params (HitComponent :type Primitive%20Component%20Object%20Reference) (OtherActor :type Actor%20Object%20Reference) (OtherComp :type Primitive%20Component%20Object%20Reference) (NormalImpulse :type Vector :default "0, 0, 0") (Hit :type Hit%20Result%20Structure%20%28by%20ref%29))
  (Game|Damage|ApplyDamage OtherActor (Variables|Default|GetDamage) 0 0))

(event EventBeginPlay)

(event Collision|EventActorBeginOverlap
  (params (OtherActor :type Actor%20Object%20Reference)))

(event EventTick
  (params (DeltaSeconds :type Float%20%28single-precision%29)))

(fn ConstructionScript
  (bind _staticmesh (Variables|Default|GetStaticMesh))
  (Transformation|SetRelativeLocation _staticmesh (Variables|Default|GetLocationOffset) false false)
  (Transformation|SetRelativeRotation _staticmesh (Variables|Default|GetRotation) false false)
  (Components|StaticMesh|SetStaticMesh (Variables|Default|GetStaticMesh) (Variables|Default|GetMesh)))