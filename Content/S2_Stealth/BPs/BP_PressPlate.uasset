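; Pressure plate that sinks while the player character stands on it and triggers a linked actor.
; Box overlap plays a timeline forward on entry and in reverse on exit, lerping the cube between its starting location and a lowered point with sweep.
; The timeline's Finished output calls TriggerMessage on TriggerableActor, so it fires at the end of travel in either direction.
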(event OnComponentBeginOverlap(Box)
  (params (OverlappedComponent :type Primitive%20Component%20Object%20Reference) (OtherActor :type Actor%20Object%20Reference) (OtherComp :type Primitive%20Component%20Object%20Reference) (OtherBodyIndex :type Integer) (bFromSweep :type Boolean) (SweepResult :type Hit%20Result%20Structure%20%28by%20ref%29))
  (if (== OtherActor (Game|GetPlayerCharacter 0))
    (bind _height (Timeline|Timeline Play)
      (:Update
        (Transformation|SetRelativeLocation (Variables|Default|GetCube) (Math|Vector|Lerp(Vector) (Variables|Default|GetStarting%20location) (Variables|Default|GetLowest%20location) _height) true false))
      (:Finished
        (Class|BPITrigger|Trigger(Message) (Variables|Default|GetTriggerableActor))))))

(event OnComponentEndOverlap(Box)
  (params (OverlappedComponent :type Primitive%20Component%20Object%20Reference) (OtherActor :type Actor%20Object%20Reference) (OtherComp :type Primitive%20Component%20Object%20Reference) (OtherBodyIndex :type Integer))
  (if (== OtherActor (Game|GetPlayerCharacter 0))
    (bind _height (Timeline|Timeline Reverse)
      (:Update
        (Transformation|SetRelativeLocation (Variables|Default|GetCube) (Math|Vector|Lerp(Vector) (Variables|Default|GetStarting%20location) (Variables|Default|GetLowest%20location) _height) true false))
      (:Finished
        (Class|BPITrigger|Trigger(Message) (Variables|Default|GetTriggerableActor))))))

(event EventBeginPlay
  (bind _output_get (Variables|Default|SetStarting%20location (Variables|/Script/Engine.SceneComponent|GetRelativeLocation (Variables|Default|GetCube))))
  (Variables|Default|SetLowest%20location (- _output_get (Math|Vector|MakeVector 0.0 0.0 (Variables|Default|GetLowest%20point)))))

(event Collision|EventActorBeginOverlap
  (params (OtherActor :type Actor%20Object%20Reference)))

(event EventTick
  (params (DeltaSeconds :type Float%20%28single-precision%29)))

(fn ConstructionScript)