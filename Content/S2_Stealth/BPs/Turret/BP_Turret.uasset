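; BP_Turret is a stealth-game turret that rotates on patrol while scanning for the player character.
; Each Tick, Detect sphere-traces forward from the Detector component, sets CurrentState based on whether the player is hit, and prints debug info.
; Without a detection, Patrol yaws the skeletal mesh at RotationSpeed; a detection halts rotation.
; FollowTarget holds interpolated look-at rotation logic but is not called in this graph.
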(event EventBeginPlay)

(event Collision|EventActorBeginOverlap
  (params (OtherActor :type Actor%20Object%20Reference)))

(event EventTick
  (params (DeltaSeconds :type Float%20%28single-precision%29))
  (bind _detected (CallFunction|Detect))
  (if (not _detected)
    (CallFunction|Patrol)))

(fn ConstructionScript)

(fn Detect
  (bind _detector (Variables|Default|GetDetector))
  (bind _returnvalue (Transformation|GetWorldLocation _detector))
  (bind (_outhit _returnvalue_2) (Collision|SphereTraceByChannel _returnvalue (+ _returnvalue (* (Math|Vector|GetForwardVector _detector) (Variables|Default|GetDetectDistance))) 1e+01 "TraceTypeQuery3" false 0 "ForOneFrame"))
  (Development|PrintText (Utilities|Text|ToText(Float) (.Distance (Collision|BreakHitResult _outhit)) "HalfToEven") true true "(R=0.000000,G=0.660000,B=1.000000,A=1.000000)" 2.0 "Distance detection")
  (if (== (.HitActor (Collision|BreakHitResult _outhit)) (Game|GetPlayerCharacter 0))
    (Development|PrintText "Found player" true true "(R=0.000000,G=0.660000,B=1.000000,A=1.000000)" 2.0 "Detection")
    (Variables|Default|SetCurrentState "NewEnumerator1")
    (return _returnvalue_2 (Game|GetPlayerCharacter 0))
    (else
      (Development|PrintText (Utilities|Text|ToText(Object) (.HitActor (Collision|BreakHitResult _outhit))) true true "(R=0.000000,G=0.660000,B=1.000000,A=1.000000)" 2.0 "Detection")
      (Variables|Default|SetCurrentState "NewEnumerator0")
      (return false 0))))

(fn Patrol
  (Transformation|AddRelativeRotation (Variables|Default|GetSkeletalMesh) (Math|Rotator|MakeRotator 0.0 0.0 (* (Utilities|Time|GetWorldDeltaSeconds) (Variables|Default|GetRotation%20speed))) false false))

(fn FollowTarget
  (params (Target :type Actor%20Object%20Reference))
  (Transformation|AddRelativeRotation (Variables|Default|GetSkeletalMesh) (Math|Interpolation|RInterpTo (.rotation (Transformation|GetRelativeTransform (Variables|Default|GetSkeletalMesh))) (Math|Rotator|FindLookatRotation (Transformation|GetActorLocation) (Transformation|GetActorLocation Target)) (Utilities|Time|GetWorldDeltaSeconds) (Variables|Default|GetRotation%20speed)) false false))