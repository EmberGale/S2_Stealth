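; BP_Collectible is a pickup that animates in place and is collected when the player character touches it.
; A Timeline started on BeginPlay drives the mesh's vertical bob and emissive material parameter, each scaled by a variable.
; The construction script sizes the trigger sphere from PickRadius.
; On player overlap it updates the collectables message through the GameInstance, spawns an explosion effect, destroys itself and plays a 2D sound.
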(event OnComponentBeginOverlap(Sphere)
  (params (OverlappedComponent :type Primitive%20Component%20Object%20Reference) (OtherActor :type Actor%20Object%20Reference) (OtherComp :type Primitive%20Component%20Object%20Reference) (OtherBodyIndex :type Integer) (bFromSweep :type Boolean) (SweepResult :type Hit%20Result%20Structure%20%28by%20ref%29))
  (if (== OtherActor (Game|GetPlayerCharacter 0))
    (Class|BPIGameInstance|UpdateCollectables(Message) (Game|GetGameInstance) (Variables|Default|GetChange))
    (Effects|SpawnEmitteratLocation "/Game/StarterContent/Particles/P_Explosion.P_Explosion" (Transformation|GetWorldLocation (Variables|Default|GetSphere)) "0, 0, 0" "0.500000,0.500000,0.500000")
    (Actor|DestroyActor)
    (Audio|PlaySound2D "/Game/Game_Item/Destruction/Wav/ExplosiveBarrelC14.ExplosiveBarrelC14" 1.0 1.0 0.0 0 0)))

(event EventBeginPlay
  (bind (_direction _z _emissive) (Timeline|Timeline Play)
    (:Update
      (Transformation|SetRelativeLocation (Variables|Default|GetMesh) (Math|Vector|MakeVector 0.0 0.0 (* _z (Variables|Default|GetWoble))) true false)
      (Rendering|Material|SetScalarParameterValueonMaterials (Variables|Default|GetMesh) "Emissive" (* _emissive (Variables|Default|GetEmissiveMult))))))

(fn ConstructionScript
  (Components|Sphere|SetSphereRadius (Variables|Default|GetSphere) (Variables|Default|GetPickRadius) true))