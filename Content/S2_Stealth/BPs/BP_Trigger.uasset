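; BP_Trigger is a box trigger actor in the stealth section that relays a trigger signal to a list of other actors.
; When its Trigger event is called while Active, it calls TriggerMessage on every entry in ActorsToTrigger.
; The construction script sizes the box from length, height and depth values, halved into extents.
; The graph has no overlap logic, so Trigger must be called from elsewhere.
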(event EventBeginPlay)

(event Collision|EventActorBeginOverlap
  (params (OtherActor :type Actor%20Object%20Reference)))

(event EventTick
  (params (DeltaSeconds :type Float%20%28single-precision%29)))

(event EventTrigger
  (if (Variables|Default|GetActive)
    (for _array_element (Variables|Default|GetActorsToTrigger)
      (Class|BPITrigger|Trigger(Message) _array_element))))

(fn ConstructionScript
  (Components|Box|SetBoxExtent (Variables|Default|GetBox) (/ (Math|Vector|MakeVector (Variables|Default|GetTriggerLength) (Variables|Default|GetTriggerHeight) (Variables|Default|GetTriggerDepth)) "2.000000,2.000000,2.000000") true))