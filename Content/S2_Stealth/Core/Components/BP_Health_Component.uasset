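; Health component for the stealth game that tracks its owner's health and signals death through OnDeath.
; It binds to the owner's OnTakeAnyDamage, passes Damage unnegated into the additive ChangeHealth, and calls OnDeath when health is at or below zero.
; Setters clamp health between zero and MaxHealth.
; BeginPlay and every change notify player 0's HUD via UpdateHealthMessage, regardless of owner.
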(event Custom|OnTakeAnyDamage_Event
  (params (DamagedActor :type Actor%20Object%20Reference) (Damage :type Float%20%28single-precision%29) (DamageType :type Damage%20Type%20Object%20Reference) (InstigatedBy :type Controller%20Object%20Reference) (DamageCauser :type Actor%20Object%20Reference))
  (Development|PrintText "Health damage")
  (CallFunction|ChangeHealth Damage)
  (if (<= (Variables|Default|GetHealth) 0.0)
    (Default|CallOnDeath)))

(event EventBeginPlay
  (EventDispatchers|AssignOnTakeAnyDamage (Components|GetOwner) (delegate Custom|OnTakeAnyDamage_Event))
  (CallFunction|UpdateUIHealth))

(fn GetHealth
  (return (Variables|Default|GetHealth)))

(fn SetHealth
  (params (Health :type Float%20%28double-precision%29))
  (Variables|Default|SetHealth (Math|Float|Clamp(Float) Health 0.0 (Variables|Default|GetMaxHealth)))
  (CallFunction|UpdateUIHealth))

(fn ChangeHealth
  (params (Delta :type Float%20%28double-precision%29))
  (Variables|Default|SetHealth (Math|Float|Clamp(Float) (+ Delta (Variables|Default|GetHealth)) 0.0 (Variables|Default|GetMaxHealth)))
  (CallFunction|UpdateUIHealth))

(fn GetMaxHealth
  (return (Variables|Default|GetMaxHealth)))

(fn UpdateUIHealth
  (Class|BPIHUD|UpdateHealth(Message) (HUD|GetHUD (Game|GetPlayerController 0))))