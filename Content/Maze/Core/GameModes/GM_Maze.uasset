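; GM_Maze is the game mode for the maze game, keeping a count of collectables.
; On BeginPlay it switches the first player controller to game-only input and flushes pending input.
; An AddCollectable event increments the count, with getter and setter functions exposing it.
; GameOver is an empty stub.
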(event Custom|AddCollectable
  (bind _result (Math|Integer|IncrementInt (Variables|Default|GetCollectables))
    (:%20%20
      (Variables|Default|SetCollectables _result))))

(event EventBeginPlay
  (Input|SetInputModeGameOnly (Game|GetPlayerController 0) true))

(fn ConstructionScript)

(fn GetCollectable
  (return (Variables|Default|GetCollectables)))

(fn SetCollectable
  (params (Collectables :type Integer))
  (Variables|Default|SetCollectables Collectables))

(fn GameOver)