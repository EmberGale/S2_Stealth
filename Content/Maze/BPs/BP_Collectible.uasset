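; BP_Collectible is a pickup in the maze game, collected when BP_MazeCharacter overlaps its sphere, whose radius is set from PickRadius at construction.
; A timeline started on BeginPlay bobs the mesh vertically and drives its Emissive material parameter, both scaled by variables.
; On pickup it passes Change to GI_Maze through UpdateCollectablesMessage, then spawns an explosion effect, destroys itself and plays a 2D sound.
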(event OnComponentBeginOverlap(Sphere)
  (params (OverlappedComponent :type Primitive%20Component%20Object%20Reference) (OtherActor :type Actor%20Object%20Reference) (OtherComp :type Primitive%20Component%20Object%20Reference) (OtherBodyIndex :type Integer) (bFromSweep :type Boolean) (SweepResult :type Hit%20Result%20Structure%20%28by%20ref%29))
  (Utilities|Casting|CastToBP_MazeCharacter OtherActor)
  (bind _asgi_maze (Utilities|Casting|CastToGI_Maze (Game|GetGameInstance)))
  (Class|BPIGIInterface|UpdateCollectables(Message) _asgi_maze (Variables|Default|GetChange))
  (Effects|SpawnEmitteratLocation "/Game/StarterContent/Particles/P_Explosion.P_Explosion" (Transformation|GetWorldLocation (Variables|Default|GetSphere)) "0, 0, 0" "0.500000,0.500000,0.500000")
  (Actor|DestroyActor)
  (Audio|PlaySound2D "/Game/Free_UI/CUE/Modern4_Cue.Modern4_Cue" 1.0 1.0 0.0 0 0))

(event EventBeginPlay
  (bind (_direction _z _emissive) (Timeline|Timeline Play)
    (:Update
      (Transformation|SetRelativeLocation (Variables|Default|GetMesh) (Math|Vector|MakeVector 0.0 0.0 (* _z (Variables|Default|GetWoble))) true false)
      (Rendering|Material|SetScalarParameterValueonMaterials (Variables|Default|GetMesh) "Emissive" (* _emissive (Variables|Default|GetEmissiveMult))))))

(event Collision|EventActorBeginOverlap
  (params (OtherActor :type Actor%20Object%20Reference)))

(event EventTick
  (params (DeltaSeconds :type Float%20%28single-precision%29)))

(fn ConstructionScript
  (Components|Sphere|SetSphereRadius (Variables|Default|GetSphere) (Variables|Default|GetPickRadius) true))